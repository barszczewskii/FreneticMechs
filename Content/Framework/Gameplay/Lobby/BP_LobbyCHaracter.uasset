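; Lobby character Blueprint that displays a player's name, skeletal mesh and animation.
; Three MC_ events, named as multicasts, set the name text, swap the mesh asset on Mesh0, or play a non-looping animation on it.
; The name event goes through a SetPlayerName function, and the actor has no active BeginPlay, Tick or construction logic, so changes come only through these events.
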(event Custom|MC_SetPlayerName
  (params (PlayerName :type Text))
  (CallFunction|SetPlayerName PlayerName))

(event Custom|MC_SetCharacterMesh
  (params (NewMesh :type Skeletal%20Mesh%20Object%20Reference))
  (Components|SkeletalMesh|SetSkeletalMeshAsset (Variables|Default|GetMesh_0) NewMesh))

(event Custom|MC_PlayMeshAnimation
  (params (NewAnimToPlay :type Animation%20Asset%20Object%20Reference))
  (Components|Animation|PlayAnimation (Variables|Default|GetMesh_0) NewAnimToPlay false))

(event EventBeginPlay)

(event Collision|EventActorBeginOverlap
  (params (OtherActor :type Actor%20Object%20Reference)))

(event EventTick
  (params (DeltaSeconds :type Float%20%28single-precision%29)))

(fn ConstructionScript)

(fn SetPlayerName
  (params (PlayerName :type Text))
  (Rendering|Components|TextRender|SetText (Variables|Default|GetPlayerName) PlayerName)
  (return))