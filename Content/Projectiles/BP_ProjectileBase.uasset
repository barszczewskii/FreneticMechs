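; Base projectile actor that launches toward an assigned Target at a set speed and gravity, optionally homing on it.
; BeginPlay configures the ProjectileMovement component when Target is valid.
; On a Box hit, the server notifies hit handlers and applies fixed damage.
; A multicast-style hit event, skipped on dedicated servers, selects particles and sound by physical surface type, prints the material name, and destroys the actor.
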(event OnComponentHit(Box)
  (params (HitComponent :type Primitive%20Component%20Object%20Reference) (OtherActor :type Actor%20Object%20Reference) (OtherComp :type Primitive%20Component%20Object%20Reference) (NormalImpulse :type Vector :default "0, 0, 0") (Hit :type Hit%20Result%20Structure%20%28by%20ref%29))
  (bind (_bblockinghit _binitialoverlap _time _distance _location _impactpoint _normal _impactnormal _physmat _hitactor) (Collision|BreakHitResult Hit))
  (Networking|SwitchHasAuthority
    (:Authority
      (Default|CallOnProjectileHit OtherActor)
      (CallFunction|MCProjectileHit true _location _normal (Class|MaterialInterface|GetPhysicalMaterial (Rendering|Material|GetMaterial OtherComp 0)) 0 "SurfaceType_Default")
      (Game|Damage|ApplyDamage _hitactor 1.5e+02 0 self))))

(event Custom|ROS_ProjectileHit
  (params (Target :type Self%20Object%20Reference))
  (CallFunction|MCProjectileHit Target false "0, 0, 0" "0, 0, 0" 0 0 "SurfaceType_Default")
  (CallFunction|ROSProjectileHit))

(event Custom|MC_ProjectileHit
  (params (Hit :type Boolean) (Hit%20Location :type Vector) (Hit%20Normal :type Vector) (PhysicalMaterial :type Physical%20Material%20Object%20Reference) (OtherActor :type Actor%20Object%20Reference%20%28by%20ref%29) (Selection :type EPhysicalSurface%20Enum :default "SurfaceType_Default"))
  (bind _returnvalue (Math|Conversions|RotationFromXVector Hit%20Normal))
  (bind _returnvalue_2 (Math|Rotator|Delta(Rotator) _returnvalue "90.000000,0.000000,0.000000"))
  (if (not (Networking|IsDedicatedServer))
    (Development|PrintString (Utilities|GetDisplayName PhysicalMaterial))
    (switch Utilities|FlowControl|Switch|SwitchonEPhysicalSurface (Variables|/Script/PhysicsCore.PhysicalMaterial|GetSurfaceType PhysicalMaterial)
      (:SurfaceType_Default
        (Effects|SpawnEmitteratLocation (Variables|EffectsCategory|GetImpactEffect) (.ImpactPoint (Collision|BreakHitResult (stale OnComponentHit(Box) Hit))))
        (Effects|SpawnEmitteratLocation "/Game/Realistic_Starter_VFX_Pack_Vol2/Particles/Hit/P_Asphalt.P_Asphalt" (.ImpactPoint (Collision|BreakHitResult (stale OnComponentHit(Box) Hit))) _returnvalue_2 "0.400000,0.400000,0.400000" false)
        (Audio|PlaySoundatLocation (Variables|Sounds|GetImpactSound) (.ImpactPoint (Collision|BreakHitResult (stale OnComponentHit(Box) Hit))) "0, 0, 0" 1.0 1.0 0.0 0 0 0 0)
        (Actor|DestroyActor))
      (:SurfaceType1
        (Effects|SpawnEmitteratLocation 0 (.ImpactPoint (Collision|BreakHitResult (stale OnComponentHit(Box) Hit))) _returnvalue_2)
        (Audio|PlaySoundatLocation 0 (.ImpactPoint (Collision|BreakHitResult (stale OnComponentHit(Box) Hit))) "0, 0, 0" 1.0 1.0 0.0 0 0 0 0)
        (Actor|DestroyActor))
      (:SurfaceType2
        (Effects|SpawnEmitteratLocation 0 (.ImpactPoint (Collision|BreakHitResult (stale OnComponentHit(Box) Hit))) _returnvalue_2)
        (Audio|PlaySoundatLocation 0 (.ImpactPoint (Collision|BreakHitResult (stale OnComponentHit(Box) Hit))) "0, 0, 0" 1.0 1.0 0.0 0 0 0 0)
        (Actor|DestroyActor))
      (:SurfaceType3
        (Effects|SpawnEmitteratLocation 0 "0, 0, 0" _returnvalue_2)
        (Audio|PlaySoundatLocation 0 "0, 0, 0" "0, 0, 0" 1.0 1.0 0.0 0 0 0 0)
        (Actor|DestroyActor)))))

(event Custom|RotateToTarget
  (Variables|/Script/Engine.MovementComponent|SetVelocity (Variables|Default|GetProjectileMovement) (* (Math|Vector|GetUnitDirection(Vector) (Transformation|GetActorLocation) (Transformation|GetActorLocation (Variables|Target|GetTarget))) (Variables|ProjectileSetttings|GetSpeed))))

(event Custom|ROS_BeginPlay)

(event EventBeginPlay
  (bind _projectilemovement (Variables|Default|GetProjectileMovement))
  (Collision|IgnoreActorwhenMoving (Variables|Default|GetBox) 0 true)
  (Collision|IgnoreActorwhenMoving (Variables|Default|GetBox) 0 true)
  (Variables|Target|GetTarget
    (:then
      (CallFunction|RotatetoTarget)
      (Variables|/Script/Engine.ProjectileMovementComponent|SetInitialSpeed _projectilemovement (Variables|ProjectileSetttings|GetSpeed))
      (Variables|/Script/Engine.ProjectileMovementComponent|SetMaxSpeed _projectilemovement (Variables|ProjectileSetttings|GetSpeed))
      (Variables|/Script/Engine.ProjectileMovementComponent|SetProjectileGravityScale _projectilemovement (Variables|ProjectileSetttings|GetGravity))
      (Variables|Target|GetTarget
        (:then
          (if (Variables|Default|Get%20IsHoming)
            (Variables|/Script/Engine.ProjectileMovementComponent|SetbIsHomingProjectile _projectilemovement true)
            (Variables|/Script/Engine.ProjectileMovementComponent|SetHomingTargetComponent _projectilemovement (Variables|/Script/Engine.Actor|GetRootComponent (Variables|Target|GetTarget)))))
        (:else)))
    (:else)))

(fn ConstructionScript)